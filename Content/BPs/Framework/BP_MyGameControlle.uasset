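; BP_MyGameControlle is a player controller that sets up input and keeps the on-screen score.
; On BeginPlay it adds an Enhanced Input mapping context, then creates WBP_MyWidget, stores it and adds it to the viewport.
; UpdateScore increments Score by one and writes it directly into the widget's ScoreNum text; nothing in this Blueprint calls it.
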(event `self.ReceiveBeginPlay`
  ; Incializar controles mediante el "input system"
  (`EnhancedInputSubsystemInterface.AddMappingContext` (subsystem `EnhancedInputLocalPlayerSubsystem`) "/Game/BPs/Inputs/MapingContext.MapingContext" 0 (struct))
  (bind _returnvalue (`|CreateWidget` "/Game/BPs/UI/WBP_MyWidget.WBP_MyWidget_C" self))
  (bind _output_get (set `self.MyWidget` _returnvalue))
  (`UserWidget.AddToViewport` _output_get 0))

(fn `UpdateScore`
  (bind _output_get (set `self.Score` (+ (`self.Score`) 1)))
  ;[0.2433 0.445 0.5448] Imprime en el widget
  (`TextBlock.SetText` (`/Game/BPs/UI/WBP_MyWidget.ScoreNum` (`self.MyWidget`)) (`KismetTextLibrary.Conv_StringToText` (`KismetStringLibrary.Concat_StrStr` "Score: " (`KismetStringLibrary.Conv_IntToString` _output_get)))))

(fn `UserConstructionScript`)