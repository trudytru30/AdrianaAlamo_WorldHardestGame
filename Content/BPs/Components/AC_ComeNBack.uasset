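; AC_ComeNBack is an actor component that moves its owner back and forth.
; A looping timer started on BeginPlay negates Direction every Duration seconds.
; Tick offsets the owner in local space by Speed and Direction scaled by delta time, without sweep, so the movement ignores collision.
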(event `self.ReceiveBeginPlay`
  ;[0.6922 0.4325 0.5454] Timer para cambiar direccion
  (`KismetSystemLibrary.K2_SetTimerDelegate` (delegate `OnTimerEnds`) (`self.Duration`) true))

(event `OnTimerEnds`
  ;[0.6922 0.4325 0.5454] Timer para cambiar direccion
  (set `self.Direction` (* (`self.Direction`) -1.0)))

(event `self.ReceiveTick`
  (params (DeltaSeconds :type "Float (single-precision)"))
  ; Mover
  (`Actor.K2_AddActorLocalOffset` (`self.GetOwner`) (* DeltaSeconds (`self.Speed`) (`self.Direction`)) false false))