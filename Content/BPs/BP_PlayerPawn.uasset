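; Player pawn that moves around, collects coins and respawns when it touches anything else.
; MoveAction applies a normalized, speed and delta-time scaled, swept local offset.
; Overlapping a BP_Coins destroys it and calls UpdateScore on BP_MyGameControlle; any other overlap returns the pawn to the PlayerStart location cached at BeginPlay.
; PrintTimer and several transform and vector nodes are unconnected practice code that never runs.
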(event `EnhancedInput|/Game/BPs/Inputs/MoveAction`
  (params (ActionValue :type "Vector2D Structure") (ElapsedSeconds :type "Float (double-precision)") (TriggeredSeconds :type "Float (double-precision)") (InputAction :type "InputAction Object Reference" :default "/Game/BPs/Inputs/MoveAction.MoveAction"))
  ; Se ejecuta cuando se realiza la accion del controller
  (:`Triggered`
    (`self.K2_AddActorLocalOffset` (* (`KismetMathLibrary.Normal2D` ActionValue) (`GameplayStatics.GetWorldDeltaSeconds`) (`self.Speed`)) true)))

(event `self.ReceiveActorEndOverlap`
  (params (OtherActor :type "Actor Object Reference"))
  ; Es como OnTriggerExit
)

(event `self.ReceiveActorBeginOverlap`
  (params (OtherActor :type "Actor Object Reference"))
  ; Es como OnTriggerEnter
  ; Si es moneda suma contador si no reinicia
  (bind _asbp_coins (cast `/Game/BPs/BP_Coins` OtherActor)
    (:`then`
      (`self.OnCoin` _asbp_coins))
    (:`CastFailed`
      (`self.OnDeath`))))

(event `self.ReceiveBeginPlay`
  (bind _returnvalue (`GameplayStatics.GetActorOfClass` "/Script/Engine.PlayerStart"))
  (set `self.InitLocation` (`self.K2_GetActorLocation` _returnvalue)))

(fn `OnCoin`
  (params (ActorToDestroy :type "Actor Object Reference"))
  ; Cuando se destruye llama a la funcion del GameController
  (`self.K2_DestroyActor` ActorToDestroy)
  (bind _asbp_my_game_controlle (cast `/Game/BPs/Framework/BP_MyGameControlle` (`self.GetController`)))
  (`/Game/BPs/Framework/BP_MyGameControlle.UpdateScore` _asbp_my_game_controlle))

(fn `OnDeath`
  ; Resetea a posicion
  (`self.K2_SetActorLocation` (`self.InitLocation`)))

(fn `PrintTimer`
  (params (Delta :type "Float (double-precision)"))
  ;[0.7615 0.3196 0.634 0.5] Logica de incremento +3 de un timer
  (bind _output_get (set `self.MyPoint` (+ (* Delta 3.0) (`self.MyPoint`))))
  (`KismetSystemLibrary.PrintString` (`KismetStringLibrary.Conv_DoubleToString` _output_get)))

(fn `UserConstructionScript`)